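; Speed power-up pickup that gives an overlapping GetGnomedCharacter a temporary boost through its IncreaseSpeed function.
; On overlap it calls IncreaseSpeed with a higher value, hides itself, waits on a retriggerable delay, then calls it again to restore speed and destroys itself.
; A SpeedupActive flag blocks repeat triggers, but it is set before the cast, so any other overlapping actor leaves the pickup locked.
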(event `self.ReceiveActorBeginOverlap`
  (params (OtherActor :type "Actor Object Reference"))
  (if (`self.Speedup active`)
    (`KismetSystemLibrary.PrintString` "Speedup already active")
    (else
      (set `self.Speedup active` true)
      (bind _asget_gnomed_character (cast `GetGnomedCharacter` OtherActor)
        (:`then`
          (`GetGnomedCharacter.IncreaseSpeed` _asget_gnomed_character 2.0)
          (`self.SetActorHiddenInGame` true)
          (`KismetSystemLibrary.PrintString` "speed increased")
          (`KismetSystemLibrary.RetriggerableDelay` 15.0)
          (bind _asget_gnomed_character_2 (cast `GetGnomedCharacter` OtherActor)
            (:`then`
              (`GetGnomedCharacter.IncreaseSpeed` _asget_gnomed_character_2 1.0)
              (set `self.Speedup active` false)
              (`KismetSystemLibrary.PrintString` "Speed Decreased")
              (`self.K2_DestroyActor`))
            (:`CastFailed`
              (`KismetSystemLibrary.PrintString` "2nd cast failed"))))
        (:`CastFailed`
          (`KismetSystemLibrary.PrintString` "cast failed"))))))

(fn `UserConstructionScript`)