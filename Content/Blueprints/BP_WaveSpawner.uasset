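; BP_WaveSpawner is a wave actor that, in this graph, only pushes wave time and enemy count to the first-person character's HUD.
; On BeginPlay it takes the HUD widget from the player pawn, retrying each tick until that widget is valid.
; Tick compares both wave values with cached copies and updates the timer or resets the gnome display only on change.
; No spawning logic appears here.
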(event `self.ReceiveBeginPlay`
  (`self.SetupHudWidget`))

(event `SetupHudWidget`
  (bind _asbp_first_person_character (cast `/Game/FirstPerson/Blueprints/BP_FirstPersonCharacter` (`GameplayStatics.GetPlayerPawn` 0)))
  (bind _hud_widget (`/Game/FirstPerson/Blueprints/BP_FirstPersonCharacter.HUD Widget` _asbp_first_person_character))
  (`/Engine/EditorBlueprintResources/StandardMacros.IsValid` _hud_widget
    (:`Is Valid`
      (set `self.HUD Widget` _hud_widget)
      (`KismetSystemLibrary.PrintString` "HUD SETUP SUCCESS" false false (struct :`G` 1.0 :`B` 0.035104 :`A` 1.0) 5.0))
    (:`Is Not Valid`
      (`KismetSystemLibrary.DelayUntilNextTick`)
      (`self.SetupHudWidget`))))

(event `self.ReceiveTick`
  (params (DeltaSeconds :type "Float (single-precision)"))
  (`/Engine/EditorBlueprintResources/StandardMacros.IsValid` (`self.HUD Widget`)
    (:`Is Valid`
      (`self.Time`)
      (`self.Enemies`))
    (:`Is Not Valid`
      (`KismetSystemLibrary.PrintString` "HUD IS INVALID" true true (struct :`R` 1.0 :`B` 0.020229 :`A` 1.0) 0.1))))

(event `Time`
  (if (!= (`self.PrevTotalTime`) (`self.TotalTimeThisWave`))
    (bind _output_get (set `self.PrevTotalTime` (`self.TotalTimeThisWave`)))
    (`/Game/Blueprints/UI/HUD_Widgets.UpdateTotalTime` (`self.HUD Widget`) _output_get)))

(event `Enemies`
  (if (!= (`self.enemiesThisWave`) (`self.PrevTotalEnemies`))
    (bind _output_get (set `self.PrevTotalEnemies` (`self.enemiesThisWave`)))
    (`/Game/Blueprints/UI/HUD_Widgets.ResetGnomes` (`self.HUD Widget`) _output_get)))

(fn `UserConstructionScript`)