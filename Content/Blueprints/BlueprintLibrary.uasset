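; Blueprint function library of small shared gameplay helpers for actor rotation, camera shake and sound.
; Spin yaws an actor's root component in local space by DeltaTime times Speed.
; Shake starts BP_CameraShake at a given scale on player 0's camera manager and returns both the manager and the shake instance.
; PlaySound plays a supplied sound at an actor's location.
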(fn `Play Sound`
  (params (Audio :type "SoundBase Object Reference") (Actor :type "Actor Object Reference"))
  (`GameplayStatics.PlaySoundAtLocation` null Audio (`Actor.K2_GetActorLocation` Actor) (struct) 1.0 1.0 0.0 null null null null))

(fn `Shake`
  (params (Scale :type "Float (double-precision)"))
  (returns (CameraManager :type "PlayerCameraManager Object Reference") (Shake :type "CameraShakeBase Object Reference"))
  (locals (HitShake :type "CameraShakeBase Object Reference") (CameraManager :type "PlayerCameraManager Object Reference"))
  (bind _returnvalue (`PlayerCameraManager.StartCameraShake` :`self` (`GameplayStatics.GetPlayerCameraManager` null) :`ShakeClass` "/Game/Blueprints/BP_CameraShake.BP_CameraShake_C" :`Scale` Scale))
  (return (`GameplayStatics.GetPlayerCameraManager` null) _returnvalue))

(fn `Spin`
  (params (ActorToSpin :type "Actor Object Reference") (DeltaTime :type "Float (double-precision)") (Speed :type "Float (double-precision)"))
  (`SceneComponent.K2_AddLocalRotation` (`Actor.RootComponent` ActorToSpin) (`KismetMathLibrary.MakeRotator` 0.0 0.0 (* DeltaTime Speed)) false false))