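; BP_SunMoon is a light actor that acts as either the sun or the moon for the level.
; On BeginPlay it waits two ticks, then reads IsNight from BP_GetGnomedGameMode and passes it to the MoonSun event.
; MoonSun applies the matching intensity, color and actor transform from its sun or moon variables and prints a debug message.
; Play start is the only trigger in this graph, with no gradual transition.
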(event `self.ReceiveBeginPlay`
  (`KismetSystemLibrary.DelayUntilNextTick`)
  (`KismetSystemLibrary.DelayUntilNextTick`)
  (bind _asbp_get_gnomed_game_mode (cast `/Game/Blueprints/BP_GetGnomedGameMode` (`GameplayStatics.GetGameMode`)))
  (`self.MoonSun` (`GetGnomedGameMode.isNight` _asbp_get_gnomed_game_mode)))

(event `MoonSun`
  (params (isMoon :type Boolean))
  (bind _lightcomponent (`self.LightComponent`))
  (bind _lightcomponent_2 (`self.LightComponent`))
  (if isMoon
    (`LightComponent.SetIntensity` _lightcomponent_2 (`self.MoonIntensity`))
    (`LightComponent.SetLightColor` _lightcomponent_2 (`KismetMathLibrary.Conv_ColorToLinearColor` (`self.MoonColor`)) true)
    (`self.K2_SetActorTransform` (`self.MoonPosition`))
    (`KismetSystemLibrary.PrintText` "Moon Updated")
    (else
      (`LightComponent.SetIntensity` _lightcomponent (`self.SunIntensity`))
      (`LightComponent.SetLightColor` _lightcomponent (`KismetMathLibrary.Conv_ColorToLinearColor` (`self.SunColor`)) true)
      (`self.K2_SetActorTransform` (`self.SunPosition`))
      (`KismetSystemLibrary.PrintText` "Sun Updated"))))

(fn `UserConstructionScript`)