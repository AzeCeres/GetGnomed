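; BP_Pickup_Ammo is a timed, spinning ammo pickup.
; When an actor tagged Player overlaps it, it finds a BP_RiflePickup via GetActorOfClass, adds ammo to that actor's TPWeapon and destroys itself.
; If uncollected, it waits after BeginPlay, blinks through a looped hide/show countdown driven by Flashes, then despawns.
; Tick yaws the static mesh at a frame-rate-independent speed.
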(event `self.ReceiveBeginPlay`
  ;[1 1 1] Delay, Flash, Destroy
  (`KismetSystemLibrary.Delay` 10.0)
  (if (> (`self.Flashes`) 0) :!label _label
    (`/Engine/EditorBlueprintResources/StandardMacros.DecrementInt` (`self.Flashes`)
      (:`  `
        (`self.SetActorHiddenInGame` true)
        (`KismetSystemLibrary.Delay` 0.2)
        (`self.SetActorHiddenInGame` false)
        (`KismetSystemLibrary.Delay` 0.2)
        (goto _label)))
    (else
      (`self.K2_DestroyActor`))))

(event `self.ReceiveActorBeginOverlap`
  (params (OtherActor :type "Actor Object Reference"))
  ;[1 1 1] Overlap, Cast to Player
  (bind _output_get (set `self.OverlapedActor` OtherActor))
  (if (`self.ActorHasTag` _output_get "Player")
    (bind _returnvalue (`GameplayStatics.GetActorOfClass` "/Game/Blueprints/BP_RiflePickup.BP_RiflePickup_C"))
    (`TP_WeaponComponent.AddAmmo` (`/Game/Blueprints/BP_RiflePickup.TP_Weapon` _returnvalue) 6)
    (`self.K2_DestroyActor`)))

(event `self.ReceiveTick`
  (params (DeltaSeconds :type "Float (single-precision)"))
  ;[1 1 1] Rotate
  (`SceneComponent.K2_AddLocalRotation` (`self.StaticMesh`) (`KismetMathLibrary.MakeRotator` 0.0 0.0 (* DeltaSeconds 45.0)) false false))

(fn `UserConstructionScript`)