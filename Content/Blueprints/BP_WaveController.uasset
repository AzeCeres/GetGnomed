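; BP_WaveController relays the current wave number and living enemy ("gnome") count to the player's HUD.
; On BeginPlay it fetches the HUD widget from BP_FirstPersonCharacter, retrying each tick until it is valid.
; Tick then polls GetEnemyCount and GetWave, neither defined here, and updates the widget only when a cached value changes.
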(event `self.ReceiveBeginPlay`
  (`self.SetupHUD`))

(event `SetupHUD`
  (bind _returnvalue (`GameplayStatics.GetActorOfClass` "/Game/FirstPerson/Blueprints/BP_FirstPersonCharacter.BP_FirstPersonCharacter_C"))
  (bind _hud_widget (`/Game/FirstPerson/Blueprints/BP_FirstPersonCharacter.HUD Widget` _returnvalue))
  (`/Engine/EditorBlueprintResources/StandardMacros.IsValid` _hud_widget
    (:`Is Valid`
      (set `self.HUD Widget` _hud_widget)
      (`KismetSystemLibrary.PrintString` "HUD SETUP SUCCESS" true true (struct :`G` 1.0 :`B` 0.035104 :`A` 1.0) 5.0))
    (:`Is Not Valid`
      (`KismetSystemLibrary.DelayUntilNextTick`)
      (`self.SetupHUD`))))

(event `self.ReceiveTick`
  (params (DeltaSeconds :type "Float (single-precision)"))
  (`/Engine/EditorBlueprintResources/StandardMacros.IsValid` (`self.HUD Widget`)
    (:`Is Valid`
      (`self.EnemiesWC`)
      (`self.Wave`))
    (:`Is Not Valid`
      (`KismetSystemLibrary.PrintString` "HUD IS INVALID" true true (struct :`R` 1.0 :`B` 0.020229 :`A` 1.0) 0.1))))

(event `EnemiesWC`
  (bind _returnvalue (`self.GetEnemyCount`))
  (if (!= _returnvalue (`self.PrevAliveEnemies`))
    (bind _output_get (set `self.PrevAliveEnemies` _returnvalue))
    (`/Game/Blueprints/UI/HUD_Widgets.UpdateGnomes` (`self.HUD Widget`) _output_get)
    (`KismetSystemLibrary.PrintString` "Updated Gnomes")))

(event `Wave`
  (bind _returnvalue (`self.GetWave`))
  (if (!= _returnvalue (`self.PrevWave`))
    (bind _output_get (set `self.PrevWave` _returnvalue))
    (`/Game/Blueprints/UI/HUD_Widgets.UpdateWave` (`self.HUD Widget`) _output_get)
    (`KismetSystemLibrary.PrintString` "Updated Wave")))

(fn `SetupHudWidget`)

(fn `UserConstructionScript`)