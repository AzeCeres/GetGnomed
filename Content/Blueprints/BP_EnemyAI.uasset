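; Gnome enemy character that chases the player, attacks in melee and dies to bullet hits.
; Tick drives an AI MoveTo on the player; on arrival a timer-gated montage plays and a line trace damages the player.
; Bullet hits subtract the player's damage stat and briefly swap the material.
; Death swaps in an impulse-driven physics shattered mesh, notifies the WaveController, randomly drops a power-up, then destroys the actor.
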(event `self.ReceiveTick`
  (params (DeltaSeconds :type "Float (single-precision)"))
  ;[1 1 1] Tick (Attack Timer Reset + Follow Player)
  (`self.FollowPlayer`)
  (set `self.attackTimer` (+ DeltaSeconds (`self.attackTimer`))))

(event `FollowPlayer`
  (bind _returnvalue (`GameplayStatics.GetPlayerPawn` 0))
  ;[1 1 1] Follow Player
  (if (not (`self.isDead`))
    (`|AIMoveTo` self (0.0 0.0 0.0) (`GameplayStatics.GetPlayerPawn` 0) 70.0
      (:`OnSuccess`
        ;[1 1 1] Attack Animation
        (if (<= (`self.attackBuffer`) (`self.attackTimer`))
          (bind _returnvalue_2 (`self.PlayAnimMontage` "/Game/LevelPrototyping/Meshes/GardenGnome/ReimportAnimation/GnomeAttackMontage.GnomeAttackMontage"))
          ;[1 1 1] Attack functionality (Timer, Line Tracer, Cast Damage to the Player)
          (set `self.attackTimer` (- 0.0 _returnvalue_2))
          (`KismetSystemLibrary.PrintText` "Attacked" false false)
          (bind _outhit (`KismetSystemLibrary.LineTraceSingle` :`Start` (`SceneComponent.GetSocketLocation` (`self.Attack Begin`) "None") :`End` (`SceneComponent.GetSocketLocation` (`self.Attack End`) "None") :`TraceChannel` "TraceTypeQuery2" :`bTraceComplex` true :`DrawDebugType` "ForDuration"))
          (bind (_bblockinghit _binitialoverlap _time _distance _location _impactpoint _normal _impactnormal _physmat _hitactor) (`GameplayStatics.BreakHitResult` _outhit))
          (`/Engine/EditorBlueprintResources/StandardMacros.IsValid` _hitactor
            (:`Is Valid`
              (if (`self.ActorHasTag` _hitactor "Player")
                (if (not (`self.isDead`))
                  (bind _asget_gnomed_character (cast `GetGnomedCharacter` _returnvalue))
                  (`GetGnomedCharacter.GetHit` _asget_gnomed_character 1)
                  (`KismetSystemLibrary.PrintText` "Player was hit" false false (struct :`R` 1.0 :`G` 0.191609 :`A` 1.0))
                  (bind _asget_gnomed_character_2 (cast `GetGnomedCharacter` _returnvalue))
                  (bind _returnvalue_3 (`GetGnomedCharacter.GetHealth` _asget_gnomed_character_2))
                  (`KismetSystemLibrary.PrintString` (`KismetStringLibrary.Conv_IntToString` _returnvalue_3) false false (struct :`R` 1.0 :`B` 0.14371 :`A` 1.0) 5.0)))))
          (else
            (`KismetSystemLibrary.PrintText` "Wanted to attack, but Coudn't" false false (struct :`R` 0.598958 :`G` 0.863646 :`B` 1.0 :`A` 0.411) 0.1)))))))

(event `TakeDamage`
  ;[1 1 1] Take Damage
  (bind _asget_gnomed_character (cast `GetGnomedCharacter` (`GameplayStatics.GetPlayerPawn` 0)))
  (bind _output_get (set `self.Health` (- (`self.Health`) (`GetGnomedCharacter.damageDealt` _asget_gnomed_character))))
  (bind _output_get_2 (set `self.isDead` (<= _output_get 0)))
  (if _output_get_2
    (`self.Death`)
    (`KismetSystemLibrary.PrintString` "Is Dead" false false)))

(event `DamageMaterial`
  (bind _mesh (`self.Mesh`))
  ;[1 1 1] Damage Material (Change mat when taking damage)
  (`PrimitiveComponent.SetMaterial` _mesh 0 "/Game/LevelPrototyping/Meshes/GardenGnome/DeadGnome.DeadGnome")
  (`KismetSystemLibrary.Delay` 0.1)
  (`PrimitiveComponent.SetMaterial` _mesh 0 "/Game/LevelPrototyping/Meshes/GardenGnome/GnomeTexture.GnomeTexture"))

(event `Death`
  (bind _mesh (`self.Mesh`))
  (bind _shatteredmesh (`self.ShatteredMesh`))
  ;[1 1 1] Dead
  (`ActorComponent.Deactivate` _mesh)
  (`SceneComponent.SetHiddenInGame` _mesh true false)
  (`ActorComponent.Activate` _shatteredmesh false)
  (`PrimitiveComponent.SetSimulatePhysics` _shatteredmesh true)
  (`SceneComponent.SetHiddenInGame` _shatteredmesh false true)
  (`PrimitiveComponent.SetCollisionEnabled` _shatteredmesh "QueryAndPhysics")
  (`KismetSystemLibrary.Delay` 0.075)
  (`PrimitiveComponent.SetCollisionEnabled` (`self.CapsuleComponent`) "NoCollision")
  (`KismetSystemLibrary.PrintText` "Collision removed" false false))

(event `self.ShatteredMesh.OnComponentActivated`
  (params (Component :type "ActorComponent Object Reference") (bReset :type Boolean))
  ;[1 1 1] Dead (Destroy actor after Delay, adds Impulse) (ADD COMUNICATION TO WAVE CONTROLLER THAT AI DIED)
  (`PrimitiveComponent.AddImpulse` (`self.ShatteredMesh`) (`self.Impulse`) "None" true)
  (`KismetSystemLibrary.PrintString` "ProtoAsset Activated" false false)
  (bind _returnvalue (`GameplayStatics.GetActorOfClass` "/Script/GetGnomed.WaveController"))
  (`WaveController.ControlWave` _returnvalue)
  (`self.SpawnPickup`)
  (`KismetSystemLibrary.Delay` 10.0)
  (`self.K2_DestroyActor`))

(event `self.ReceiveHit`
  (params (MyComp :type "PrimitiveComponent Object Reference") (Other :type "Actor Object Reference") (OtherComp :type "PrimitiveComponent Object Reference") (bSelfMoved :type Boolean) (HitLocation :type "Vector Structure") (HitNormal :type "Vector Structure") (NormalImpulse :type "Vector Structure") (Hit :type "HitResult Structure (by ref)"))
  ;[1 1 1] Hit by bullet
  (set `self.Impulse` NormalImpulse)
  (if (`ActorComponent.ComponentHasTag` OtherComp "Bullet")
    (if (not (== (`self.LastCollision`) OtherComp))
      (set `self.LastCollision` OtherComp)
      (`KismetSystemLibrary.PrintText` "Hit By Bullet" false false)
      (`self.TakeDamage`)
      (`self.DamageMaterial`))))

(event `SpawnPickup`
  (bind _returnvalue (`KismetMathLibrary.RandomInteger` 3))
  (bind _returnvalue_2 (`self.GetTransform`))
  (bind _newvar (`self.NewVar`))
  ;[1 1 1] Spawn Pickup
  (set `self.NewVar` (`KismetMathLibrary.MakeTransform` (`KismetMathLibrary.MakeVector` (.x (.location _returnvalue_2)) (.y (.location _returnvalue_2)) (+ (.z (.location _returnvalue_2)) 50.0)) (.rotation _returnvalue_2) (.scale _returnvalue_2)))
  (if (<= (`KismetMathLibrary.RandomFloat`) (`self.DropChance`))
    (if (== _returnvalue 0)
      (`|SpawnActorFromClass` (`self.SPDUP`) (`self.NewVar`) "AdjustIfPossibleButAlwaysSpawn" "OverrideRootScale" null null)
      (elif (== _returnvalue 1)
        (`|SpawnActorFromClass` (`self.HLTUP`) _newvar "Undefined" "OverrideRootScale" null null)
        (else
          (`|SpawnActorFromClass` (`self.DMGUP`) _newvar "Undefined" "OverrideRootScale" null null))))))

(fn `UserConstructionScript`)