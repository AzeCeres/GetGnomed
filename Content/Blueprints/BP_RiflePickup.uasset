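; Rifle pickup that attaches its TPWeapon to the player's GetGnomed character when picked up and slowly regenerates ammo.
; Tick adds one round each time the AmmoBuffer countdown expires while below max, then updates the HUD bullet count only when ammo has changed.
; Setup from BeginPlay retries on the next tick until the first-person character's HUD widget is valid, then initializes its bullet display.
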(event `self.ReceiveBeginPlay`
  (`self.SetupWeapon`))

(event `self.ReceiveTick`
  (params (DeltaSeconds :type "Float (single-precision)"))
  (bind _tp_weapon (`self.TP_Weapon`))
  (if (== (`TP_WeaponComponent.Ammo` _tp_weapon) (`TP_WeaponComponent.MaxAmmo` _tp_weapon))
    (set `self.AmmoTimer` (`self.AmmoBuffer`))
    (else
      (bind _output_get (set `self.AmmoTimer` (- (`self.AmmoTimer`) DeltaSeconds)))
      (if (<= _output_get 0.0)
        (set `self.AmmoTimer` (`self.AmmoBuffer`))
        (`TP_WeaponComponent.AddAmmo` (`self.TP_Weapon`) 1))))
  (`self.UpdateAmmo`))

(event `self.TP_PickUp.OnPickUp`
  (params (PickUpCharacter :type "Object Object Reference"))
  ;[1 1 1] PickUp
  (bind _asget_gnomed_character (cast `GetGnomedCharacter` (`GameplayStatics.GetPlayerPawn` 0)))
  (`TP_WeaponComponent.AttachWeapon` (`self.TP_Weapon`) _asget_gnomed_character))

(event `UpdateAmmo`
  ;[1 1 1] Update Ammo, Setups Rifle if not setup yet.
  (if (`self.isSetup`)
    (if (!= (`self.PreviousBullets`) (`TP_WeaponComponent.Ammo` (`self.TP_Weapon`)))
      (bind _output_get (set `self.PreviousBullets` (`TP_WeaponComponent.Ammo` (`self.TP_Weapon`))))
      (`/Game/Blueprints/UI/HUD_Widgets.UpdateBulletCount` (`self.HUD Widget`) _output_get))))

(event `SetupWeapon`
  ;[1 1 1] SetupRifle
  (bind _asbp_first_person_character (cast `/Game/FirstPerson/Blueprints/BP_FirstPersonCharacter` (`GameplayStatics.GetPlayerPawn` 0)))
  (bind _hud_widget (`/Game/FirstPerson/Blueprints/BP_FirstPersonCharacter.HUD Widget` _asbp_first_person_character))
  (`/Engine/EditorBlueprintResources/StandardMacros.IsValid` _hud_widget
    (:`Is Valid`
      (bind _output_get (set `self.HUD Widget` _hud_widget))
      (`/Game/Blueprints/UI/HUD_Widgets.SetupBullets` _output_get (`TP_WeaponComponent.MaxAmmo` (`self.TP_Weapon`)))
      (set `self.isSetup` true))
    (:`Is Not Valid`
      (`KismetSystemLibrary.DelayUntilNextTick`)
      (`self.SetupWeapon`))))

(fn `SetupRifle`)

(fn `UserConstructionScript`)